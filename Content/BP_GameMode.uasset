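; Game mode that registers joining players and starts the game once the expected number has joined.
; Each PostLogin increments a counter, compares it with the game instance's player count to trigger StartGame, then adds the player to BP_GameState's PlayersInfo, already marked ready.
; A delayed timer set on login later rewrites those entries to fill in each controller's possessed BP_Pawn.
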(event Custom|Check%20If%20All%20Players%20Joined
  (bind _asbp_game_instance (Utilities|Casting|CastToBP_GameInstance (Game|GetGameInstance)))
  (if (== (Variables|Default|GetPlayers%20Joined) (Variables|/Game/BP_GameInstance.BP_GameInstance_C|GetPlayers%20Of%20Game _asbp_game_instance))
    (Class|TGameMode|StartGame)))

(event Custom|Add%20Player%20Pawn%20To%20Player%20Info
  (bind _asbp_game_state (Utilities|Casting|CastToBP_GameState (Game|GetGameState)))
  (for (_array_element _array_index) (Variables|/Game/BP_GameState.BP_GameState_C|GetPlayers%20Info _asbp_game_state)
    (bind _asbp_pawn (Utilities|Casting|CastToBP_Pawn (Pawn|GetControlledPawn (.playercontroller _array_element))))
    (Utilities|Array|SetArrayElem (Variables|/Game/BP_GameState.BP_GameState_C|GetPlayers%20Info _asbp_game_state) _array_index (Utilities|Struct|MakeST_PlayerInfo (.playercontroller _array_element) _asbp_pawn (.playername _array_element) (.playerstate _array_element) (.bisready _array_element)))))

(event EventPostLogin
  (params (NewPlayer :type Player%20Controller%20Object%20Reference))
  (|CallParentFunction NewPlayer)
  (Math|Integer|IncrementInt (Variables|Default|GetPlayers%20Joined)
    (:%20%20
      (CallFunction|CheckifAllPlayersJoined)
      (bind _asbp_game_state (Utilities|Casting|CastToBP_GameState (Game|GetGameState)))
      (Utilities|Array|Add (Variables|/Game/BP_GameState.BP_GameState_C|GetPlayers%20Info _asbp_game_state) (Utilities|Struct|MakeST_PlayerInfo NewPlayer 0 (Utilities|Text|ToText(String) (Class|AdvancedSessionsLibrary|GetPlayerName NewPlayer)) (Variables|/Script/Engine.Controller|GetPlayerState NewPlayer) true))
      (Utilities|Time|SetTimerbyEvent (delegate Custom|Add%20Player%20Pawn%20To%20Player%20Info) 15.0))))

(fn ConstructionScript)