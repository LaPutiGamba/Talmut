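; Lobby player controller that shows the lobby widget and links it to the lobby game mode for player list, ready state and match start.
; Server events set the PlayerState ready flag and request list refreshes, which client events push into the widget.
; GameStart starts only with authority and all players ready, while StartGame skips the ready check.
; Kicked clients destroy their session and return to the Menu level.
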(event Custom|Server%20Set%20Is%20Ready
  (params (Is%20Ready :type Boolean))
  (bind _asbp_player_state_lobby (Utilities|Casting|CastToBP_PlayerStateLobby (Variables|GetPlayerState)))
  (Variables|/Game/BP_PlayerStateLobby.BP_PlayerStateLobby_C|SetbIsReady _asbp_player_state_lobby Is%20Ready)
  (CallFunction|ServerRequestUpdatePlayerList))

(event Custom|Client%20Got%20Kicked
  (Class|MultiplayerSessionsSubsystem|DestroySession (Subsystems|GetMultiplayerSessionsSubsystem))
  (Game|OpenLevel(byName) "Menu"))

(event Custom|Client%20Update%20Player%20List
  (params (Players%20Info :type Array%20of%20ST%20Player%20Info%20Structures))
  (Default|UpdatePlayerList (Variables|Default|GetLobby%20Widget) Players%20Info))

(event Custom|Server%20Request%20Update%20Player%20List
  (bind _asbp_game_mode_lobby (Utilities|Casting|CastToBP_GameModeLobby (Game|GetGameMode)))
  (Default|UpdatePlayerList _asbp_game_mode_lobby))

(event Custom|Start%20Game
  (Networking|SwitchHasAuthority
    (:Authority
      (bind _asbp_game_mode_lobby (Utilities|Casting|CastToBP_GameModeLobby (Game|GetGameMode)))
      (Default|StartGamefromLobby _asbp_game_mode_lobby))))

(event EventBeginPlay
  (if (Pawn|IsLocalPlayerController)
    (bind _returnvalue (UserInterface|CreateWidget "/Game/Widgets/Lobby/WBP_Lobby.WBP_Lobby_C"))
    (bind _output_get (Variables|Default|SetLobby%20Widget _returnvalue))
    (UserInterface|Viewport|AddtoViewport _output_get 0)
    (Utilities|Time|SetTimerbyFunctionName 0 "Server Request Update Player List" 0.1)))

(fn ConstructionScript)

(fn GameStart
  (Networking|SwitchHasAuthority
    (:Authority
      (bind _asbp_game_mode_lobby (Utilities|Casting|CastToBP_GameModeLobby (Game|GetGameMode)))
      (bind _is_ready (Default|IsAllPlayersReady _asbp_game_mode_lobby))
      (if _is_ready
        (Default|StartGamefromLobby _asbp_game_mode_lobby)
        (return true)
        (else
          (return false))))
    (:Remote
      (return false))))