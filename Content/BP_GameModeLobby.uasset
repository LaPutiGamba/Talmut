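; Lobby game mode that tracks connected players, checks readiness, handles kicks and launches the match by server travel to the Main map.
; Login and logout maintain the Players array; UpdatePlayerList rebuilds name and ready info from player states and sends it to every client.
; The all-ready check also stores the player count in the game instance.
; Kicking only notifies the chosen player's controller through ClientGotKicked.
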(event Custom|Start%20Game%20From%20Lobby
  (Viewport|RemoveAllWidgets)
  (Class|AdvancedSessionsLibrary|ServerTravel "/Game/Maps/Main" false false))

(event EventPostLogin
  (params (NewPlayer :type Player%20Controller%20Object%20Reference))
  (bind _asbp_player_controller_lobby (Utilities|Casting|CastToBP_PlayerControllerLobby NewPlayer))
  (Utilities|Array|Add (Variables|Default|GetPlayers) _asbp_player_controller_lobby))

(event EventOnLogout
  (params (ExitingController :type Controller%20Object%20Reference))
  (bind _asbp_player_controller_lobby (Utilities|Casting|CastToBP_PlayerControllerLobby ExitingController))
  (Utilities|Array|RemoveItem (Variables|Default|GetPlayers) _asbp_player_controller_lobby)
  (CallFunction|UpdatePlayerList))

(fn ConstructionScript)

(fn UpdatePlayerList
  (Utilities|Array|Clear (Variables|Default|GetPlayers%20Info))
  (for _array_element (Variables|Default|GetPlayers)
    (bind _asbp_player_state_lobby (Utilities|Casting|CastToBP_PlayerStateLobby (Variables|/Script/Engine.Controller|GetPlayerState _array_element)))
    (Utilities|Array|Add (Variables|Default|GetPlayers%20Info) (Utilities|Struct|MakeST_PlayerInfo _array_element (Utilities|Text|ToText(String) (Class|AdvancedSessionsLibrary|GetPlayerName _array_element)) _asbp_player_state_lobby (Variables|/Game/BP_PlayerStateLobby.BP_PlayerStateLobby_C|GetbIsReady _asbp_player_state_lobby))))
  (for _array_element_2 (Variables|Default|GetPlayers)
    (Default|ClientUpdatePlayerList _array_element_2 (Variables|Default|GetPlayers%20Info))))

(fn IsAllPlayersReady
  (bind _asbp_game_instance (Utilities|Casting|CastToBP_GameInstance (Game|GetGameInstance)))
  (bind _output_get (Variables|/Game/BP_GameInstance.BP_GameInstance_C|SetPlayers%20Of%20Game _asbp_game_instance 0))
  (LocalVariables|SetbAllPlayersReady true)
  (for _array_element (Variables|Default|GetPlayers)
    (bind _asbp_player_state_lobby (Utilities|Casting|CastToBP_PlayerStateLobby (Variables|/Script/Engine.Controller|GetPlayerState _array_element)))
    (if (Variables|/Game/BP_PlayerStateLobby.BP_PlayerStateLobby_C|GetbIsReady _asbp_player_state_lobby)
      _
      (else
        (LocalVariables|SetbAllPlayersReady false)))
    (Math|Integer|IncrementInt _output_get))
  (return (LocalVariables|GetbAllPlayersReady)))

(fn KickPlayer
  (params (Player%20Index :type Integer))
  (Default|ClientGotKicked (Utilities|Array|Get(acopy) (Variables|Default|GetPlayers) Player%20Index)))